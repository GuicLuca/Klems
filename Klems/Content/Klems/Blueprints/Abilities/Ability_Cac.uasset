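; Melee ability for KS_Character that deals fixed damage to another character at close range in front of the instigator.
; On start, it runs the parent logic, then sweeps a short box trace on the Visibility channel from the camera location along the base aim rotation.
; A KS_Character hit by the trace loses health through DecrementHealth, and the trace is debug-drawn for a duration.
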(fn `Start`
  (params (Instigator :type "Actor Object Reference"))
  (returns (ReturnValue :type Boolean))
  (bind _returnvalue (`parent.Start` Instigator))
  (bind _asks_character (cast `/Game/Klems/Blueprints/Character/KS_Character` Instigator))
  (bind _returnvalue_2 (`KSCharacter.GetCamera` _asks_character))
  (bind _returnvalue_3 (`SceneComponent.K2_GetComponentLocation` _returnvalue_2))
  (bind _outhit (`KismetSystemLibrary.BoxTraceSingle` :`Start` _returnvalue_3 :`End` (+ _returnvalue_3 (* (`KismetMathLibrary.GetForwardVector` (`Pawn.GetBaseAimRotation` _asks_character)) 60)) :`HalfSize` (30.0 30.0 30.0) :`TraceChannel` "TraceTypeQuery1" :`DrawDebugType` "ForDuration"))
  (bind _asks_character_2 (cast `/Game/Klems/Blueprints/Character/KS_Character` (`.HitActor` (`GameplayStatics.BreakHitResult` _outhit))))
  (`KSCharacter.DecrementHealth` _asks_character_2 50.0)
  (return _returnvalue))