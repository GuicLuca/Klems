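; Reload ability for KS_Character that refills the character's ammo through the combat component.
; On start it calls Reload on the KSCombatComponent and plays the reloading montage, with a debug print.
; On stop it sets the combat component's ammo to a hard-coded full amount and removes the Reloading effect tag from the instigator's ability component.
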(fn `Start`
  (params (Instigator :type "Actor Object Reference"))
  (returns (ReturnValue :type Boolean))
  (bind _returnvalue (`parent.Start` Instigator))
  (bind _asks_character (cast `/Game/Klems/Blueprints/Character/KS_Character` Instigator))
  (`KismetSystemLibrary.PrintString` "rechargement")
  (`KSCombatComponent.Reload` (`Actor.GetComponentByClass` _asks_character "/Script/Klems.KSCombatComponent"))
  (`Character.PlayAnimMontage` _asks_character "/Game/Externals/SoldierAnim/Stand/reloading_Montage.reloading_Montage" 1.0 "None")
  (return _returnvalue))

(fn `Stop`
  (params (Instigator :type "Actor Object Reference"))
  (returns (ReturnValue :type Boolean))
  (bind _returnvalue (`parent.Stop` Instigator))
  (set `KSCombatComponent.Ammo` 10 (`Actor.GetComponentByClass` Instigator "/Script/Klems.KSCombatComponent"))
  (`BlueprintGameplayTagLibrary.RemoveGameplayTag` (`ASAbilityComponent.ActiveGameplayTags` (`Actor.GetComponentByClass` Instigator "/Script/AbilitySystem.ASAbilityComponent")) (struct :`TagName` "Ability.Effect.Reloading"))
  (return _returnvalue))