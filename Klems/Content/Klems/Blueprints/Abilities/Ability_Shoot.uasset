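; Shoot ability that fires a hitscan from a KS_Character instigator's camera and modifies the health of the character it hits.
; Start runs the parent logic, then sphere-traces a thin, long line along the camera's forward vector on the Visibility channel, with debug drawing left on.
; A hit KS_Character receives Modifier_Health on the Life.Health attribute of its ASAttributeSetComponent.
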(fn `Start`
  (params (Instigator :type "Actor Object Reference"))
  (returns (ReturnValue :type Boolean))
  (bind _returnvalue (`parent.Start` Instigator))
  (bind _asks_character (cast `/Game/Klems/Blueprints/Character/KS_Character` Instigator))
  (bind _returnvalue_2 (`KSCharacter.GetCamera` _asks_character))
  (bind _returnvalue_3 (`SceneComponent.K2_GetComponentLocation` _returnvalue_2))
  (bind _outhit (`KismetSystemLibrary.SphereTraceSingle` :`Start` _returnvalue_3 :`End` (+ _returnvalue_3 (* (`SceneComponent.GetForwardVector` _returnvalue_2) 10000)) :`Radius` 2.0 :`TraceChannel` "TraceTypeQuery1" :`DrawDebugType` "ForDuration"))
  (bind _asks_character_2 (cast `/Game/Klems/Blueprints/Character/KS_Character` (`.HitActor` (`GameplayStatics.BreakHitResult` _outhit)))
    (:`then`
      (bind _returnvalue_4 (`ASAttributeSetComponent.GetAttribute` (`Actor.GetComponentByClass` _asks_character_2 "/Script/AbilitySystem.ASAttributeSetComponent") (struct :`TagName` "Attribute.Life.Health")))
      (`ASAttribute.AddModifier` _returnvalue_4 "/Game/Klems/Blueprints/Modifiers/Modifier_Health.Modifier_Health_C"))
    (:`CastFailed`
      _))
  (return _returnvalue))