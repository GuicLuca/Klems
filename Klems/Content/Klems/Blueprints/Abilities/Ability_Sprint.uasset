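; Sprint ability that raises the instigator's movement speed attribute through a modifier while active.
; Start calls the parent, then adds Modifier_Sprint to Attribute.Movement.Speed on the instigator's ASAttributeSetComponent.
; Stop calls the parent, then removes the modifier by the Modifier.Movement.Run tag rather than by class.
; Both print a debug string and succeed only if the parent call and the modifier change succeed.
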(fn `Start`
  (params (Instigator :type "Actor Object Reference"))
  (returns (ReturnValue :type Boolean))
  (`KismetSystemLibrary.PrintString` "Run started")
  (bind _returnvalue (`parent.Start` Instigator))
  (bind _returnvalue_2 (`ASAttributeSetComponent.AddModifier` (`Actor.GetComponentByClass` Instigator "/Script/AbilitySystem.ASAttributeSetComponent") (struct :`TagName` "Attribute.Movement.Speed") "/Game/Klems/Blueprints/Modifiers/Modifier_Sprint.Modifier_Sprint_C"))
  (return (and _returnvalue_2 _returnvalue)))

(fn `Stop`
  (params (Instigator :type "Actor Object Reference"))
  (returns (ReturnValue :type Boolean))
  (`KismetSystemLibrary.PrintString` "Run stoped")
  (bind _returnvalue (`parent.Stop` null))
  (bind _returnvalue_2 (`ASAttributeSetComponent.RemoveModifier` (`Actor.GetComponentByClass` Instigator "/Script/AbilitySystem.ASAttributeSetComponent") (struct :`TagName` "Attribute.Movement.Speed") (struct :`TagName` "Modifier.Movement.Run")))
  (return (and _returnvalue_2 _returnvalue)))