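; Player character for a shooter with infection, handling weapons, HUD, animation and death.
; BeginPlay spawns separate third-person and first-person guns for CombatComponent, adds input mapping and creates score and in-game widgets.
; Shoot, reload, ammo and hit events play montages, switching to mutant attacks at full InfectionDensity, while StopInfection swaps both meshes to zombie animation and destroys the guns.
; Die possesses a new spectator pawn and has the server travel to the lobby when no players remain.
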(event `self.ReceiveBeginPlay`
  (bind _tabui (`self.TabUI`))
  (`parent.ReceiveBeginPlay`)
  (bind _returnvalue (`|SpawnActorFromClass` "/Game/Klems/Blueprints/Weapon/BP_Weapon.BP_Weapon_C" (`KismetMathLibrary.MakeTransform` (0.0 0.0 0.0)) "Undefined" "OverrideRootScale" null null))
  (set `self.TPSGun` _returnvalue)
  (bind _returnvalue_2 (`|SpawnActorFromClass` "/Game/Klems/Blueprints/Weapon/BP_WeaponFPS.BP_WeaponFPS_C" (`KismetMathLibrary.MakeTransform` (0.0 0.0 0.0)) "Undefined" "OverrideRootScale" null null))
  (set `self.FPSGun` _returnvalue_2)
  (`KSCombatComponent.Init` (`self.CombatComponent`) self)
  (`KSCombatComponent.EquipWeapon` (`self.CombatComponent`) _returnvalue _returnvalue_2)
  (bind _asplayer_controller (cast `PlayerController` (`self.GetController`)))
  (`EnhancedInputSubsystemInterface.AddMappingContext` (pcsubsystem `EnhancedInputLocalPlayerSubsystem` _asplayer_controller) "/Game/Klems/Inputs/MappingContexts/IMC_KSDefault.IMC_KSDefault" 0 (struct))
  (bind _returnvalue_3 (`|CreateWidget` "/Game/Klems/Blueprints/Widgets/HUD/WBP_Score.WBP_Score_C"))
  (set `self.TabUI` _returnvalue_3)
  (`UserWidget.AddToViewport` _tabui 0)
  (`Widget.SetRenderOpacity` _tabui 0.0)
  (bind _returnvalue_4 (`|CreateWidget` "/Game/Klems/Blueprints/Widgets/HUD/WBP_In_Game.WBP_In_Game_C"))
  (set `self.InGameWidget` _returnvalue_4)
  (`UserWidget.AddToViewport` _returnvalue_4 0)
  (set `/Game/Klems/Blueprints/Widgets/HUD/WBP_In_Game.OwningPlayer` self _returnvalue_4))

(event `self.OnAmmoChanged`
  (params (OldValue :type Integer) (NewValue :type Integer))
  (if (>= (`self.InfectionDensity`) 1.0)
    (if (== NewValue 0)
      (`|PlayMontage` (`self.Mesh`) "/Game/Externals/ZombieAnim/Actions/Mutant_Punch_Montage.Mutant_Punch_Montage"))
    (elif (== NewValue -1)
      (`|PlayMontage` (`self.Mesh`) "/Game/Externals/SoldierAnim/Stand/reloading_Montage.reloading_Montage")
      (elif (not (== NewValue 10))
        (`|PlayMontage` (`self.Mesh`) "/Game/Externals/SoldierAnim/Stand/AS_firePistol_Montage2.AS_firePistol_Montage2" 0.5)))))

(event `self.ShowTabUI`
  (`Widget.SetRenderOpacity` (`self.TabUI`) 1.0))

(event `self.HideTabUI`
  (`Widget.SetRenderOpacity` (`self.TabUI`) 0.0))

(event `self.TakeHit`
  (`|PlayMontage` (`self.Mesh`) "/Game/Externals/SoldierAnim/Stand/hit_reaction_Montage.hit_reaction_Montage"))

(event `self.Shoot`
  (`/Engine/EditorBlueprintResources/StandardMacros.DoOnce` false :!label _label
    (:`Completed`
      (`|ExecutionSequence`
        (:`then_0`
          (if (>= (`self.InfectionDensity`) 1.0)
            (bind _returnvalue (`self.GetFPSMesh`))
            (`|PlayMontage` _returnvalue "/Game/Externals/ZombieAnim/FPS/FPS_Mutant_Attack_Montage.FPS_Mutant_Attack_Montage")
            (else
              (bind _returnvalue_2 (`self.GetFPSMesh`))
              (`|PlayMontage` _returnvalue_2 "/Game/Externals/SoldierAnim/FPS/FPS_Shoot_Montage.FPS_Shoot_Montage"))))
        (:`then_1`
          (`KismetSystemLibrary.Delay` 0.5)
          (goto _label :!via `Reset`))))))

(event `self.stopInfection`
  (`SkinnedMeshComponent.SetSkinnedAssetAndUpdate` (`self.Mesh`) "/Game/Externals/Zombie/Survivor_A_Lusth.Survivor_A_Lusth" true)
  (`SkeletalMeshComponent.SetAnimInstanceClass` (`self.Mesh`) "/Game/Externals/ZombieAnim/AB_Zombie.AB_Zombie_C")
  (bind _returnvalue (`self.GetFPSMesh`))
  (`SkinnedMeshComponent.SetSkinnedAssetAndUpdate` _returnvalue "/Game/Externals/Zombie/Survivor_A_Lusth.Survivor_A_Lusth" true)
  (`SkeletalMeshComponent.SetAnimInstanceClass` _returnvalue "/Game/Externals/ZombieAnim/FPS/AB_FPS_Zombie.AB_FPS_Zombie_C")
  (`self.K2_DestroyActor` (`self.TPSGun`))
  (`self.K2_DestroyActor` (`self.FPSGun`)))

(event `self.Reload`
  (bind _returnvalue (`self.GetFPSMesh`))
  (`|PlayMontage` _returnvalue "/Game/Externals/SoldierAnim/Stand/reloading_Montage.reloading_Montage"))

(event `self.Die`
  (bind _returnvalue (`self.GetLocalViewingPlayerController`))
  (`Widget.RemoveFromParent` (`self.InGameWidget`))
  (`self.RemoveTPSGun`)
  (`self.K2_DestroyActor` (`self.FPSGun`))
  (`self.K2_DestroyActor`)
  (`|ExecutionSequence`
    (:`then_0`
      (bind _outactors (`GameplayStatics.GetAllActorsOfClass` "KS_Character_C"))
      (if (<= (`KismetArrayLibrary.Array_Length` _outactors) 1)
        (`KismetSystemLibrary.PrintString` "Plus de jouers")
        (`/Engine/EditorBlueprintResources/ActorMacros.Switch Has Authority`
          (:`Authority`
            (`self.OpenLobby`)))))
    (:`then_1`
      (`Controller.UnPossess` _returnvalue)
      (bind _returnvalue_2 (`|SpawnActorFromClass` "/Game/Klems/Blueprints/SpectatorCam/BP_Spectator.BP_Spectator_C" (`self.GetTransform`) "AlwaysSpawn" "OverrideRootScale" _returnvalue null))
      (`Controller.Possess` _returnvalue _returnvalue_2))))

(event `RemoveTPSGun`
  (`self.K2_DestroyActor` (`self.TPSGun`)))

(event `OpenLobby`
  (`KismetSystemLibrary.ExecuteConsoleCommand` "ServerTravel LVL_Lobby" null))

(fn `UserConstructionScript`)