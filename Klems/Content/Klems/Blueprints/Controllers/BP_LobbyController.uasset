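; Player controller for the multiplayer lobby that manages lobby UI, ready status and leaving the session.
; On BeginPlay the local controller switches to cursor-driven UI-only input, and events lazily create the lobby and match-starting widgets, hiding the former for the latter.
; Ready changes go to BP_LobbyGamemode, while UpdatePlayerReady refreshes the lobby widget's ready label.
; EndClientSession destroys the session and opens the menu level.
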(event `self.ReceiveBeginPlay`
  (if (`self.IsLocalController`)
    (set `self.bShowMouseCursor` true)
    (`WidgetBlueprintLibrary.SetInputMode_UIOnlyEx` self null)))

(event `EndClientSession`
  (`DestroySessionCallbackProxy.DestroySession` self
    (:`then`
      (`GameplayStatics.OpenLevelBySoftObjectPtr` "/Game/Klems/Levels/Menus/LVL_Menu.LVL_Menu"))))

(event `CreateMatchStartingMenu`
  (`self.UI_ShowMatchStartMenu`))

(event `CreateLobbyMenu`
  (`self.UI_ShowLobbyMenu`))

(event `ServerUpdatePLayerReady`
  (params (isReady :type Boolean))
  (bind _asbp_lobby_gamemode (cast `/Game/Klems/Blueprints/GameModes/BP_LobbyGamemode` (`GameplayStatics.GetGameMode`)))
  (`/Game/Klems/Blueprints/GameModes/BP_LobbyGamemode.PLayerChangerStatus` _asbp_lobby_gamemode self isReady))

(event `UpdatePlayerReady`
  (params (isPlayersReady :type "Array of Boolean"))
  (bind _hud_lobby (`self.HUD_Lobby`))
  (`/Engine/EditorBlueprintResources/StandardMacros.IsValid` _hud_lobby
    (:`Is Valid`
      (`/Game/Klems/Blueprints/Widgets/Lobby/WBP_Lobby.SetLabelNBPlayersReay` _hud_lobby isPlayersReady))))

(fn `UI_ShowLobbyMenu`
  (`/Engine/EditorBlueprintResources/StandardMacros.IsValid` (`self.HUD_Lobby`)
    (:`Is Valid`
      _)
    (:`Is Not Valid`
      (bind _returnvalue (`|CreateWidget` "/Game/Klems/Blueprints/Widgets/Lobby/WBP_Lobby.WBP_Lobby_C" self))
      (set `self.HUD_Lobby` _returnvalue)))
  (`UserWidget.AddToViewport` (`self.HUD_Lobby`) 0)
  (return))

(fn `UI_ShowMatchStartMenu`
  (`/Engine/EditorBlueprintResources/StandardMacros.IsValid` (`self.HUD_Lobby`)
    (:`Is Valid`
      (`Widget.SetVisibility` (`self.HUD_Lobby`) "Hidden"))
    (:`Is Not Valid`
      _))
  (`/Engine/EditorBlueprintResources/StandardMacros.IsValid` (`self.HUD_MatchStart`)
    (:`Is Valid`
      _)
    (:`Is Not Valid`
      (bind _returnvalue (`|CreateWidget` "/Game/Klems/Blueprints/Widgets/Lobby/WBP_MatchStart.WBP_MatchStart_C" self))
      (set `self.HUD_MatchStart` _returnvalue)))
  (`UserWidget.AddToViewport` (`self.HUD_MatchStart`) 0)
  (return))

(fn `UserConstructionScript`)