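; Player controller for the results screen, showing player names and scores at the end of a match.
; On begin play, the local controller shows the cursor and switches to UI-only input.
; UpdateHUD passes names and scores to a WBP_ResultScreen widget, first creating it and adding it to the viewport if missing.
; EndClientSession destroys the online session, then opens the main menu level.
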(event `self.ReceiveBeginPlay`
  (if (`self.IsLocalController`)
    (set `self.bShowMouseCursor` true)
    (`WidgetBlueprintLibrary.SetInputMode_UIOnlyEx` self null)))

(event `EndClientSession`
  (`DestroySessionCallbackProxy.DestroySession` self
    (:`then`
      (`GameplayStatics.OpenLevelBySoftObjectPtr` "/Game/Klems/Levels/Menus/LVL_Menu.LVL_Menu"))))

(event `CreateHUD`
  (`/Engine/EditorBlueprintResources/StandardMacros.IsValid` (`self.HUD`)
    (:`Is Valid`
      _)
    (:`Is Not Valid`
      (bind _returnvalue (`|CreateWidget` "/Game/Klems/Blueprints/Widgets/Menu/ResultScreen/WBP_ResultScreen.WBP_ResultScreen_C" self))
      (set `self.HUD` _returnvalue)))
  (`UserWidget.AddToViewport` (`self.HUD`) 0))

(event `UpdateHUD`
  (params (Names :type "Array of String") (Scores :type "Array of Integer"))
  (`/Engine/EditorBlueprintResources/StandardMacros.IsValid` (`self.HUD`) :!label _label
    (:`Is Valid`
      (`/Game/Klems/Blueprints/Widgets/Menu/ResultScreen/WBP_ResultScreen.FillResultScreen` (`self.HUD`) Names Scores))
    (:`Is Not Valid`
      (`self.CreateHUD`)
      (goto _label))))

(fn `UserConstructionScript`)