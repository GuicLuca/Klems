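; Deathmatch game mode that tracks the player count and, shortly after BeginPlay, starts every BP_ScrollWall.
; On each death, a DoOnce with delayed reset gates the authority-side countdown, filtering near-simultaneous calls.
; When one player or fewer remains, it disables the first remaining character's input, scores it in BP_GSDeathMatch and shows scores on every player controller.
; It also spawns possessed spectators and serves per-player scoreboard show/hide requests.
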(event `self.HandleStartingNewPlayer`
  (params (NewPlayer :type "PlayerController Object Reference"))
  (`parent.HandleStartingNewPlayer` NewPlayer)
  (`/Engine/EditorBlueprintResources/StandardMacros.IncrementInt` (`self.NbPlayers`)) ; On new connection, increment the number of present player
)

(event `self.ReceiveBeginPlay`
  (`KismetSystemLibrary.Delay` 5.0)
  (`self.StartGame`))

(event `StartGame`
  (bind _outactors (`GameplayStatics.GetAllActorsOfClass` "/Game/Klems/Blueprints/ScrollingWall/BP_ScrollWall.BP_ScrollWall_C"))
  (for _array_element _outactors
    (`/Game/Klems/Blueprints/ScrollingWall/BP_ScrollWall.Start` _array_element)))

(event `PlayerDies`
  (params (RemainingPlayers :type "Array of Pawn Object Reference"))
  (bind _output (`|GetArrayItem` RemainingPlayers))
  (`/Engine/EditorBlueprintResources/StandardMacros.DoOnce` false :!label _label
    (:`Completed`
      (`/Engine/EditorBlueprintResources/ActorMacros.Switch Has Authority`
        (:`Authority`
          (bind _result (`/Engine/EditorBlueprintResources/StandardMacros.DecrementInt` (`self.NbPlayers`))
            (:`  `
              (if (<= _result 1)
                (bind _asks_character (cast `/Game/Klems/Blueprints/Character/KS_Character` _output))
                (`self.DisableInput` _asks_character (`Pawn.GetLocalViewingPlayerController` _asks_character))
                (bind _asbp_gsdeath_match (cast `/Game/Klems/Blueprints/GameStates/BP_GSDeathMatch` (`GameplayStatics.GetGameState`)))
                (`/Game/Klems/Blueprints/GameStates/BP_GSDeathMatch.AddScore` _asbp_gsdeath_match (`Pawn.PlayerState` _output))
                (bind (_playersnames _playersscores) (`self.MapToArrays` (`/Game/Klems/Blueprints/GameStates/BP_GSDeathMatch.Scores` _asbp_gsdeath_match)))
                (`self.DisplayScores` _playersnames _playersscores))
              (`KismetSystemLibrary.Delay` 0.1)
              (goto _label :!via `Reset`))))))))

(event `DisplayScores`
  (params (PlayersNames :type "Array of String") (PlayersScores :type "Array of Integer"))
  (bind _asbp_gsdeath_match (cast `/Game/Klems/Blueprints/GameStates/BP_GSDeathMatch` (`GameplayStatics.GetGameState`)))
  (for _array_element (`GameStateBase.PlayerArray` _asbp_gsdeath_match)
    (bind _asbp_pcdeath_match (cast `/Game/Klems/Blueprints/Controllers/BP_PCDeathMatch` (`PlayerState.GetPlayerController` _array_element)))
    (`/Game/Klems/Blueprints/Controllers/BP_PCDeathMatch.ShowTabPanel` _asbp_pcdeath_match PlayersNames PlayersScores)))

(event `SpawnSpectator`
  (params (Controller :type "Controller Object Reference") (Transform :type "Transform Structure"))
  (`/Engine/EditorBlueprintResources/StandardMacros.IsValid` Controller
    (:`Is Valid`
      (`/Engine/EditorBlueprintResources/ActorMacros.Switch Has Authority`
        (:`Authority`
          (bind _returnvalue (`|SpawnActorFromClass` "/Game/Klems/Blueprints/SpectatorCam/BP_Spectator.BP_Spectator_C" Transform "Undefined" "OverrideRootScale" null null))
          (`Controller.Possess` Controller _returnvalue))))))

(event `ServerShowTabPanel`
  (params (Instigator :type "/Game/Klems/Blueprints/Controllers/BP_PCDeathMatch Object Reference"))
  (bind _asbp_gsdeath_match (cast `/Game/Klems/Blueprints/GameStates/BP_GSDeathMatch` (`GameplayStatics.GetGameState`)))
  (bind (_playersnames _playersscores) (`self.MapToArrays` (`/Game/Klems/Blueprints/GameStates/BP_GSDeathMatch.Scores` _asbp_gsdeath_match)))
  (`/Game/Klems/Blueprints/Controllers/BP_PCDeathMatch.ShowTabPanel` Instigator _playersnames _playersscores))

(event `self.K2_OnLogout`
  (params (ExitingController :type "Controller Object Reference"))
  (`/Engine/EditorBlueprintResources/StandardMacros.DecrementInt` (`self.NbPlayers`)))

(event `ServerHideTabPanel`
  (params (Instigator :type "/Game/Klems/Blueprints/Controllers/BP_PCDeathMatch Object Reference"))
  (`/Game/Klems/Blueprints/Controllers/BP_PCDeathMatch.HideTabPanel` Instigator))

(fn `MapToArrays`
  (params (Scores :type "Map of String to Integer"))
  (returns (PlayersNames :type "Array of String") (PlayersScores :type "Array of Integer"))
  (locals (tmpScores :type "Array of Integer") (tmpPlayers :type "Array of String"))
  (bind _keys (`BlueprintMapLibrary.Map_Keys` Scores))
  (for (_array_element _array_index) _keys
    (`KismetArrayLibrary.Array_Set` (`local.tmpScores`) _array_index (`BlueprintMapLibrary.Map_Find` Scores _array_element) true))
  (return _keys (`local.tmpScores`)))

(fn `UserConstructionScript`)

(fn `WaitingForPLayers`
  (bind _asbp_gsdeath_match (cast `/Game/Klems/Blueprints/GameStates/BP_GSDeathMatch` (`GameplayStatics.GetGameState`)))
  (set `self.NbPlayers` (`KismetArrayLibrary.Array_Length` (`GameStateBase.PlayerArray` _asbp_gsdeath_match))))