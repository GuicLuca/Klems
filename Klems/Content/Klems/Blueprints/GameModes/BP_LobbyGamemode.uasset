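; Lobby game mode that tracks connected players and their ready states, then starts the match.
; Join, logout and ready changes update parallel controller and ready arrays, which are pushed to every BP_LobbyController to refresh the lobby.
; When everyone is ready, it waits briefly and rechecks so the start can be cancelled.
; It then shows each player a match-starting menu and has BP_GameInstance travel to the map with the player count.
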(event `self.HandleStartingNewPlayer`
  (params (NewPlayer :type "PlayerController Object Reference"))
  ;[1 0.4878 0.4878] New Connection
  (`KismetSystemLibrary.PrintString` "New player connection")
  (bind _returnvalue (`GameplayStatics.GetCurrentLevelName` true))
  (switch `string` _returnvalue
    (:`LVL_Lobby`
      (bind _asbp_lobby_controller (cast `/Game/Klems/Blueprints/Controllers/BP_LobbyController` NewPlayer)
        (:`then`
          (bind _returnvalue_2 (`KismetArrayLibrary.Array_Add` (`self.All_ConectedPlayers`) _asbp_lobby_controller))
          (`KismetArrayLibrary.Array_Set` (`self.isPlayerReady`) _returnvalue_2 false true)
          (`/Game/Klems/Blueprints/Controllers/BP_LobbyController.CreateLobbyMenu` _asbp_lobby_controller)
          (`self.UpdateLobby` true))
        (:`CastFailed`
          (`KismetSystemLibrary.PrintString` "Cast failed on BP_LobbyController in Event handling new player (BP_LobbyGamemode)"))))))

(event `self.K2_OnLogout`
  (params (ExitingController :type "Controller Object Reference"))
  (bind _all_conectedplayers (`self.All_ConectedPlayers`))
  ;[1 0.4878 0.4878] New Connection
  (bind _asbp_lobby_controller (cast `/Game/Klems/Blueprints/Controllers/BP_LobbyController` ExitingController))
  (`KismetArrayLibrary.Array_Remove` (`self.isPlayerReady`) (`KismetArrayLibrary.Array_Find` _all_conectedplayers _asbp_lobby_controller))
  (`KismetArrayLibrary.Array_RemoveItem` _all_conectedplayers _asbp_lobby_controller)
  (`self.UpdateLobby` true))

(event `PLayerChangerStatus`
  (params (Player :type "PlayerController Object Reference") (Ready :type Boolean))
  ;[1 0.4878 0.4878] New Connection
  (bind _asbp_lobby_controller (cast `/Game/Klems/Blueprints/Controllers/BP_LobbyController` Player))
  (`KismetArrayLibrary.Array_Set` (`self.isPlayerReady`) (`KismetArrayLibrary.Array_Find` (`self.All_ConectedPlayers`) _asbp_lobby_controller) Ready true)
  (`self.UpdateLobby` true)
  (bind _everyone_ready (`self.EveryoneReady`))
  (if _everyone_ready
    ;;[1 1 1] let a chance to cancel the match start
    (`KismetSystemLibrary.Delay` 2.0)
    (bind _everyone_ready_2 (`self.EveryoneReady`))
    (if _everyone_ready_2
      (for _array_element (`self.All_ConectedPlayers`)
        (`/Game/Klems/Blueprints/Controllers/BP_LobbyController.CreateMatchStartingMenu` _array_element))
      (bind _asbp_game_instance (cast `/Game/Klems/Blueprints/Utils/BP_GameInstance` (`GameplayStatics.GetGameInstance`))
        (:`then`
          (`/Game/Klems/Blueprints/Utils/BP_GameInstance.TravelToMap` _asbp_game_instance (`KismetArrayLibrary.Array_Length` (`self.All_ConectedPlayers`)) (`self.MapName`)))
        (:`CastFailed`
          (`KismetSystemLibrary.PrintString` "Cast failed on BP_Gameinstance in btnReadyClicked (WBP_Lobby)"))))))

(event `UpdateLobby`
  (params (PlayerStatus :type Boolean))
  (if PlayerStatus
    (for _array_element (`self.All_ConectedPlayers`)
      (`/Game/Klems/Blueprints/Controllers/BP_LobbyController.UpdatePlayerReady` _array_element (`self.isPlayerReady`)))))

(fn `EveryoneReady`
  (returns (`everyone ready` :type Boolean))
  (for _array_element (`self.isPlayerReady`)
    (if (not _array_element)
      (return _array_element)))
  (return true) ; Everyone is ready, return true
)

(fn `GetAmountOfPlayerReady`
  (returns (NBplayersReady :type Integer))
  (locals (amount :type Integer))
  (for _array_element (`self.isPlayerReady`)
    (if _array_element
      (`/Engine/EditorBlueprintResources/StandardMacros.IncrementInt` (`local.amount`))))
  (return (`local.amount`)))

(fn `UserConstructionScript`
  (`parent.UserConstructionScript`))