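; Game mode for the result screen that shows each player's name and score from the finished match.
; On BeginPlay it copies the GameInstance's Scores map into parallel name and score arrays, clears the map, then builds and fills player 0's HUD.
; Each newly joining player's result screen controller is tracked in a connected list and gets the same HUD update, and is removed on logout.
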(event `self.ReceiveBeginPlay`
  (bind _asbp_game_instance (cast `/Game/Klems/Blueprints/Utils/BP_GameInstance` (`GameplayStatics.GetGameInstance`)))
  (bind _scores (`/Game/Klems/Blueprints/Utils/BP_GameInstance.Scores` _asbp_game_instance))
  (bind _keys (`BlueprintMapLibrary.Map_Keys` _scores))
  (bind _output_get (set `self.PlayersNames` _keys))
  (for _array_element _output_get
    (`KismetArrayLibrary.Array_Set` (`self.PLayersScores`) (`KismetArrayLibrary.Array_Find` (`self.PlayersNames`) _array_element) (`BlueprintMapLibrary.Map_Find` _scores _array_element) true))
  (bind _asbp_game_instance_2 (cast `/Game/Klems/Blueprints/Utils/BP_GameInstance` (`GameplayStatics.GetGameInstance`)))
  (`BlueprintMapLibrary.Map_Clear` (`/Game/Klems/Blueprints/Utils/BP_GameInstance.Scores` _asbp_game_instance_2))
  (bind _asbp_result_screen_controller (cast `/Game/Klems/Blueprints/Controllers/BP_ResultScreenController` (`GameplayStatics.GetPlayerController` 0)))
  (`/Game/Klems/Blueprints/Controllers/BP_ResultScreenController.CreateHUD` _asbp_result_screen_controller)
  (`/Game/Klems/Blueprints/Controllers/BP_ResultScreenController.UpdateHUD` _asbp_result_screen_controller (`self.PlayersNames`) (`self.PLayersScores`)))

(event `self.HandleStartingNewPlayer`
  (params (NewPlayer :type "PlayerController Object Reference"))
  (bind _asbp_result_screen_controller (cast `/Game/Klems/Blueprints/Controllers/BP_ResultScreenController` NewPlayer))
  (`KismetArrayLibrary.Array_Add` (`self.All_ConnectedPlayers`) _asbp_result_screen_controller)
  (`/Game/Klems/Blueprints/Controllers/BP_ResultScreenController.CreateHUD` _asbp_result_screen_controller)
  (`/Game/Klems/Blueprints/Controllers/BP_ResultScreenController.UpdateHUD` _asbp_result_screen_controller (`self.PlayersNames`) (`self.PLayersScores`)))

(event `self.K2_OnLogout`
  (params (ExitingController :type "Controller Object Reference"))
  (bind _asbp_result_screen_controller (cast `/Game/Klems/Blueprints/Controllers/BP_ResultScreenController` ExitingController))
  (`KismetArrayLibrary.Array_RemoveItem` (`self.All_ConnectedPlayers`) _asbp_result_screen_controller))

(fn `UserConstructionScript`)