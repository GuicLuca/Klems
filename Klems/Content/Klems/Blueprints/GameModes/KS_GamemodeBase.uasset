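; Base game mode for Klems that gates multiplayer match start in LVL_Lobby and LVL_Map1.
; On PostLogin it resets any running countdown and, with at least two KS_Character actors present, calls ServerTravelPlayer.
; That event opens LVL_Map1 through OpenLevel with a listen option string, disables character movement and starts a looping countdown timer.
; When the countdown reaches zero, the timer clears and movement is restored for the gathered players.
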(event `self.ReceiveBeginPlay`
  (bind _returnvalue (`GameplayStatics.GetCurrentLevelName` true))
  (bind _returnvalue_2 (or (== _returnvalue "LVL_Lobby") (== _returnvalue "LVL_Map1")))
  (if _returnvalue_2
    (set `self.IsAbleToPrepareMatch` _returnvalue_2)
    (else
      (`KismetSystemLibrary.LogString` "Not yet in LVL_Lobby" false))))

(event `self.K2_PostLogin`
  (params (NewPlayer :type "PlayerController Object Reference"))
  (if (`self.IsAbleToPrepareMatch`)
    ;[0.2473 0.1997 1] If a game was already in launch and new player join, reset timer game and start new one, else create first timer game
    (if (`KismetSystemLibrary.K2_IsValidTimerHandle` (`self.TimerRef`))
      (`KismetSystemLibrary.PrintString` "A new player has joined, please wait" true true (struct :`R` 1.0 :`G` 0.432907 :`A` 1.0) 3.0)
      (set `self.ValueTimer` 3)
      (`KismetSystemLibrary.K2_ClearAndInvalidateTimerHandle` (`self.TimerRef`)))
    ;[0.2307 0.9183 1] Check if there is at minimum 2 players in game map
    (bind (_outputpin _canlaunchgame) (`self.CheckNumberOfPlayer`))
    (if _canlaunchgame
      (`self.ServerTravelPlayer`))))

(event `Timer`
  ;[0.6168 1 0.6332] Launch Match when all player are detected and in the game
  (`KismetSystemLibrary.PrintString` (`KismetStringLibrary.Concat_StrStr` "Match Start in : " (`KismetStringLibrary.Conv_IntToString` (`self.ValueTimer`))) false)
  (bind _result (`/Engine/EditorBlueprintResources/StandardMacros.DecrementInt` (`self.ValueTimer`))
    (:`  `
      (if (== _result 0)
        (`KismetSystemLibrary.K2_ClearAndInvalidateTimerHandle` (`self.TimerRef`))
        (`self.SetKSCharacterMovement` (`self.Players`))))))

(event `ServerTravelPlayer`
  (`GameplayStatics.OpenLevelBySoftObjectPtr` "/Game/Klems/Levels/Maps/LVL_Map1.LVL_Map1" true "ServerTravel LVL_Map1?listen")
  ;[1 0.2016 0.3782] Remove the ability to walk during the preparing phase for all players
  (bind _outactors (`GameplayStatics.GetAllActorsOfClass` "/Game/Klems/Blueprints/Character/KS_Character.KS_Character_C"))
  (`self.ChangeMovementModeForAllPlayers` _outactors (`self.RemoveMovement`))
  ;[0.6168 1 0.6332] Launch Match when all player are detected and in the game
  (`KismetSystemLibrary.PrintString` "Match preparing" false)
  (bind _returnvalue (`KismetSystemLibrary.K2_SetTimerDelegate` (delegate `Timer`) 1.0 true))
  (set `self.TimerRef` _returnvalue))

(event `SetKSCharacterMovement`
  (params (Players :type "Array of KSCharacter Object Reference"))
  ;[0.4251 0.3003 1] Give Abitity to Walk to Players
  (`self.ChangeMovementModeForAllPlayers` Players (`self.AddMovement`)))

(fn `ChangeMovementModeForAllPlayers`
  (params (Array :type "Array of KSCharacter Object Reference") (MovementMode :type "EMovementMode Enum" :default "MOVE_None"))
  (for _array_element Array
    (`CharacterMovementComponent.SetMovementMode` (`Character.CharacterMovement` _array_element) MovementMode 0)))

(fn `CheckNumberOfPlayer`
  (returns (OutputPin :type "Array of /Game/Klems/Blueprints/Character/KS_Character Object Reference") (CanLaunchGame :type Boolean))
  (bind _outactors (`GameplayStatics.GetAllActorsOfClass` "/Game/Klems/Blueprints/Character/KS_Character.KS_Character_C"))
  (bind _output_get (set `self.Players` _outactors))
  (return _outactors (> (`KismetArrayLibrary.Array_Length` _output_get) 1)))

(fn `UserConstructionScript`)