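; Deathmatch GameState that keeps a per-player score map and restarts the match by server travel.
; A looping one-second timer adds any new PlayerArray entries to the map at zero.
; AddScore passes through a DoOnce with no reset, so only the first call increments a score, waits five seconds and issues a ServerTravel console command for LVL_Map1.
; That command string is appended without a separating space.
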(event `self.ReceiveBeginPlay`
  (`KismetSystemLibrary.K2_SetTimer` null "WaitingForPlayers" 1.0 true))

(event `AddScore`
  (params (Player :type "PlayerState Object Reference"))
  (bind _scores (`self.Scores`))
  (`/Engine/EditorBlueprintResources/StandardMacros.DoOnce` false
    (:`Completed`
      (bind _result (`/Engine/EditorBlueprintResources/StandardMacros.IncrementInt` (`BlueprintMapLibrary.Map_Find` _scores Player))
        (:`  `
          (`BlueprintMapLibrary.Map_Add` _scores Player _result)
          (`KismetSystemLibrary.Delay` 5.0)
          (`KismetSystemLibrary.ExecuteConsoleCommand` (`KismetStringLibrary.Concat_StrStr` "ServerTravel " "LVL_Map1") null))))))

(fn `UserConstructionScript`)

(fn `WaitingForPLayers`
  (bind _scores (`self.Scores`))
  (for _array_element (`self.PlayerArray`)
    (if (not (`.ReturnValue` (`BlueprintMapLibrary.Map_Find` _scores _array_element)))
      (`BlueprintMapLibrary.Map_Add` _scores _array_element))))