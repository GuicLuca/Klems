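; Deathmatch game state that keeps per-player round wins across level reloads and ends the match when a player reaches four points.
; It loads the score map from BP_GameInstance on BeginPlay, then after a delay adds missing players by name at zero.
; AddScore increments a player's score, saves the map back to the game instance, then issues a delayed ServerTravel command targeting the map or the result screen.
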(event `self.ReceiveBeginPlay`
  (bind _scores (`self.Scores`))
  (bind _asbp_game_instance (cast `/Game/Klems/Blueprints/Utils/BP_GameInstance` (`GameplayStatics.GetGameInstance`)))
  (set `self.Scores` (`/Game/Klems/Blueprints/Utils/BP_GameInstance.Scores` _asbp_game_instance))
  (`KismetSystemLibrary.Delay` 5.0)
  (for _array_element (`self.PlayerArray`)
    (bind _returnvalue (`PlayerState.GetPlayerName` _array_element))
    (if (`.ReturnValue` (`BlueprintMapLibrary.Map_Find` _scores _returnvalue))
      (`KismetSystemLibrary.PrintString` "KeyFound")
      (else
        (`BlueprintMapLibrary.Map_Add` _scores _returnvalue)))))

(event `AddScore`
  (params (Player :type "PlayerState Object Reference"))
  (bind _returnvalue (`PlayerState.GetPlayerName` Player))
  (bind _scores (`self.Scores`))
  (bind _result (`/Engine/EditorBlueprintResources/StandardMacros.IncrementInt` (`BlueprintMapLibrary.Map_Find` _scores _returnvalue))
    (:`  `
      (`BlueprintMapLibrary.Map_Add` _scores _returnvalue _result)
      (bind _asbp_game_instance (cast `/Game/Klems/Blueprints/Utils/BP_GameInstance` (`GameplayStatics.GetGameInstance`)))
      (if (>= _result 4)
        (`KismetSystemLibrary.PrintString` (`KismetStringLibrary.Concat_StrStr` _returnvalue " wins"))
        (set `/Game/Klems/Blueprints/Utils/BP_GameInstance.Scores` (`self.Scores`) _asbp_game_instance)
        (`KismetSystemLibrary.Delay` 2.0)
        (`KismetSystemLibrary.ExecuteConsoleCommand` (`KismetStringLibrary.Concat_StrStr` "ServerTravel " "LVL_ResultScreen") null)
        (else
          (set `/Game/Klems/Blueprints/Utils/BP_GameInstance.Scores` (`self.Scores`) _asbp_game_instance)
          (`KismetSystemLibrary.Delay` 2.0)
          (`KismetSystemLibrary.ExecuteConsoleCommand` (`KismetStringLibrary.Concat_StrStr` "ServerTravel " "LVL_Map1") null))))))

(fn `UserConstructionScript`)