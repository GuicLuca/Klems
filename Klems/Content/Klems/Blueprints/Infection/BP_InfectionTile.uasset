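; BP_InfectionTile is an infection tile whose infection density grows over time.
; After an initial delay, BeginPlay starts a looping timer that calls Infect, which adds a set density increment and clears the timer once density reaches full.
; Collider overlap events are empty; the logic to start and stop infection on KSCharacter is disconnected and never runs.
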(event `self.ReceiveBeginPlay`
  (`KismetSystemLibrary.Delay` (`self.DelayBeforeInfection`))
  (bind _returnvalue (`KismetSystemLibrary.K2_SetTimer` null "Infect" (`self.TimerDelay`) true))
  (set `self.Timer` _returnvalue))

(event `self.ReceiveTick`
  (params (DeltaSeconds :type "Float (single-precision)")))

(event `self.Collider.OnComponentBeginOverlap`
  (params (OverlappedComponent :type "PrimitiveComponent Object Reference") (OtherActor :type "Actor Object Reference") (OtherComp :type "PrimitiveComponent Object Reference") (OtherBodyIndex :type Integer) (bFromSweep :type Boolean) (SweepResult :type "HitResult Structure (by ref)"))
  ;[0.1384 1 0] infection
)

(event `self.Collider.OnComponentEndOverlap`
  (params (OverlappedComponent :type "PrimitiveComponent Object Reference") (OtherActor :type "Actor Object Reference") (OtherComp :type "PrimitiveComponent Object Reference") (OtherBodyIndex :type Integer))
  ;[0.1384 1 0] infection
)

(fn `Infect`
  (`self.addInfectionDensity` (`self.InfectionDensityToAdd`))
  (if (>= (`self.InfectionDensity`) 1.0)
    (`KismetSystemLibrary.K2_ClearAndInvalidateTimerHandle` (`self.Timer`))))

(fn `UserConstructionScript`)