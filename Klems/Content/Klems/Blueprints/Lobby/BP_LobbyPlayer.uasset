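; Lobby player actor that sets up the lobby UI for the local viewing player.
; On BeginPlay it switches to UI-only input with a visible cursor and creates WBP_Lobby, showing the start button only with authority.
; It counts BP_LobbyPlayer actors and passes that number to the widget's AddPlayer; removal passes one less to the same function.
; RemoveWidget takes the UI down, while the PlayerName and Widget RepNotifies are empty.
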(event `self.ReceiveBeginPlay`
  (bind _returnvalue (`self.GetLocalViewingPlayerController`))
  (`WidgetBlueprintLibrary.SetInputMode_UIOnlyEx` _returnvalue null)
  (set `PlayerController.bShowMouseCursor` true _returnvalue)
  (bind _outactors (`GameplayStatics.GetAllActorsOfClass` "BP_LobbyPlayer_C"))
  (set `self.NbPlayers` (`KismetArrayLibrary.Array_Length` _outactors))
  (bind _returnvalue_2 (`|CreateWidget` "/Game/Klems/Blueprints/Widgets/Lobby/WBP_Lobby.WBP_Lobby_C" (`self.GetLocalViewingPlayerController`)))
  (bind _output_get (set `self.Widget` _returnvalue_2))
  (`UserWidget.AddToViewport` _output_get 0)
  (`/Engine/EditorBlueprintResources/ActorMacros.Switch Has Authority`
    (:`Authority`
      (`/Game/Klems/Blueprints/Widgets/Lobby/WBP_Lobby.ShowStartBtn` (`self.Widget`)))
    (:`Remote`
      _))
  (`self.AddPlayerToList`))

(event `AddPlayerToList`
  (`/Game/Klems/Blueprints/Widgets/Lobby/WBP_Lobby.AddPlayer` (`self.Widget`) (`self.NbPlayers`)))

(event `RemovePlayerFromList`
  (`/Game/Klems/Blueprints/Widgets/Lobby/WBP_Lobby.AddPlayer` (`self.Widget`) (- (`self.NbPlayers`) 1)))

(event `RemoveWidget`
  (`Widget.RemoveFromParent` (`self.Widget`)))

(fn `OnRep_PlayerName`)

(fn `OnRep_Widget`)

(fn `UserConstructionScript`)