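; BP_ScrollWall is a moving wall tile that infects KSCharacters while they overlap its collider.
; On BeginPlay, after an initial delay, it starts a looping timer that raises infection density until it reaches 1, then clears itself.
; The tile then teleports to Point2 and shuttles endlessly between Point1 and Point2 through chained MoveComponentTo calls.
; Collider overlap begin and end start and stop the character's infection, independent of the density value.
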(event `self.ReceiveBeginPlay`
  (bind _timetravel (`self.TimeTravel`))
  (bind _tile (`self.Tile`))
  (bind _returnvalue (`self.K2_GetActorLocation` (`self.Point2`)))
  (bind _relativerotation (`SceneComponent.RelativeRotation` _tile))
  (`KismetSystemLibrary.Delay` (`self.DelayBeforeInfection`))
  (bind _returnvalue_2 (`KismetSystemLibrary.K2_SetTimer` null "Infect" (`self.TimerDelay`) true))
  (set `self.Timer` _returnvalue_2)
  (`SceneComponent.K2_SetWorldLocation` (`self.Tile`) _returnvalue false true)
  (`KismetSystemLibrary.MoveComponentTo` _tile (`self.K2_GetActorLocation` (`self.Point1`)) _relativerotation false false _timetravel :!label _label)
  (`KismetSystemLibrary.MoveComponentTo` _tile _returnvalue _relativerotation false false _timetravel)
  (goto _label))

(event `self.Collider.OnComponentBeginOverlap`
  (params (OverlappedComponent :type "PrimitiveComponent Object Reference") (OtherActor :type "Actor Object Reference") (OtherComp :type "PrimitiveComponent Object Reference") (OtherBodyIndex :type Integer) (bFromSweep :type Boolean) (SweepResult :type "HitResult Structure (by ref)"))
  ;[0.1384 1 0] infection
  (bind _askscharacter (cast `KSCharacter` OtherActor))
  (`KSCharacter.startInfection` _askscharacter))

(event `self.Collider.OnComponentEndOverlap`
  (params (OverlappedComponent :type "PrimitiveComponent Object Reference") (OtherActor :type "Actor Object Reference") (OtherComp :type "PrimitiveComponent Object Reference") (OtherBodyIndex :type Integer))
  ;[0.1384 1 0] infection
  (bind _askscharacter (cast `KSCharacter` OtherActor))
  (`KSCharacter.stopInfection` _askscharacter))

(fn `Infect`
  (`self.addInfectionDensity` (`self.InfectionDensityToAdd`))
  (if (>= (`self.InfectionDensity`) 1.0)
    (`KismetSystemLibrary.K2_ClearAndInvalidateTimerHandle` (`self.Timer`))))

(fn `UserConstructionScript`)