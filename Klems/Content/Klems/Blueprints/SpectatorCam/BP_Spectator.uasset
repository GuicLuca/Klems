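; BP_Spectator is a spectator Blueprint that shows the deathmatch scoreboard when it begins play.
; On BeginPlay it creates a WBP_ScoresPanel widget and adds it to the viewport.
; GetScores splits the Scores map from BP_GSDeathMatch into player and score arrays.
; BeginPlay then builds its own Scores map from those arrays and passes it to DisplayScores once, with no later refresh.
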(event `self.ReceiveBeginPlay`
  (bind _returnvalue (`|CreateWidget` "/Game/Klems/Blueprints/Widgets/HUD/Scores/WBP_ScoresPanel.WBP_ScoresPanel_C"))
  (bind _output_get (set `self.ScoreWidget` _returnvalue))
  (`UserWidget.AddToViewport` _returnvalue 0)
  (`UserWidget.AddToViewport` _output_get 0)
  (`self.GetScores`)
  (for (_array_element _array_index) (`self.Players`)
    (`BlueprintMapLibrary.Map_Add` (`self.Scores`) _array_element (`KismetArrayLibrary.Array_Find` (`self.Score`) _array_index)))
  (`/Game/Klems/Blueprints/Widgets/HUD/Scores/WBP_ScoresPanel.DisplayScores` (`self.ScoreWidget`) (`self.Scores`)))

(event `GetScores`
  (bind _asbp_gsdeath_match (cast `/Game/Klems/Blueprints/GameState/BP_GSDeathMatch` (`GameplayStatics.GetGameState`)))
  (bind _scores (`/Game/Klems/Blueprints/GameState/BP_GSDeathMatch.Scores` _asbp_gsdeath_match))
  (bind _keys (`BlueprintMapLibrary.Map_Keys` _scores))
  (set `self.Players` _keys)
  (bind _values (`BlueprintMapLibrary.Map_Values` _scores))
  (set `self.Score` _values))

(fn `UserConstructionScript`)